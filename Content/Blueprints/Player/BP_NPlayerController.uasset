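; BP_NPlayerController is a player controller that links the player to the game mode and the root UI layout.
; On BeginPlay it caches the current BP_NGameMode.
; The attribute menu event pauses the game, then casts the game mode again and has it open the menu.
; GetUILayoutRoot lazily creates the WBP_OverAllLayout widget owned by this controller and returns the cached instance, without adding it to the viewport.
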(event EventBeginPlay
  (bind _asbp_ngame_mode (Utilities|Casting|CastToBP_NGameMode (Game|GetGameMode)))
  (Variables|Default|SetGameMode _asbp_ngame_mode))

(event EventTick
  (params (DeltaSeconds :type Float%20%28single-precision%29)))

(event EventOnOpenAttribueMenu
  (Game|SetGamePaused true)
  (bind _asbp_ngame_mode (Utilities|Casting|CastToBP_NGameMode (Game|GetGameMode)))
  (Class|NGameModeBase|OpenAttributeMenu _asbp_ngame_mode))

(fn ConstructionScript)

(fn GetUILayoutRoot
  (Variables|Default|GetRootUILayout
    (:then
      _)
    (:else
      (bind _returnvalue (UserInterface|CreateWidget "/Game/Blueprints/UI/CommonUI/WBP_OverAllLayout.WBP_OverAllLayout_C" self))
      (Variables|Default|SetRootUILayout _returnvalue)))
  (return (Variables|Default|GetRootUILayout)))