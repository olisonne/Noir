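; GA_MeleeAttack_Warrior is the warrior's melee attack gameplay ability, playing a random tagged attack montage from the avatar.
; On the gameplay event matching the montage's tag, it finds live players around that tag's combat socket location, excluding the avatar.
; It applies damage to each one and then ends the ability, which also ends if the montage is cancelled.
; An unconnected delayed EndAbility branch never runs.
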(event Ability|EventActivateAbility
  (bind _returnvalue (Ability|GetAvatarActorfromActorInfo))
  (Ability|CommitAbility)
  (bind _returnvalue_2 (Class|CombatInterface|GetAttackMontages(Message) (Ability|GetAvatarActorfromActorInfo)))
  (bind _output_get (Variables|Default|SetMontageData (Class|NDamageGameplayAbility|GetRandomTaggedMontagefromArray _returnvalue_2)))
  (|PlayMontageandWaitProxy "None" (.Montage (Utilities|Struct|BreakTaggedMontage _output_get)) 1.0 "None" true 1.0 0.0 false
    (:then
      (Ability|Tasks|WaitGameplayEvent (.MontageTag (Utilities|Struct|BreakTaggedMontage _output_get)) 0
        (:EventReceived
          (bind _returnvalue_3 (Class|CombatInterface|GetCombatSocketLocation(Message) _returnvalue (.MontageTag (Utilities|Struct|BreakTaggedMontage _output_get))))
          (bind _outoverlappingactors (Class|NAbilityFunctionLibrary|GetLivePlayersWithinRadius _returnvalue (Utilities|Array|MakeArray _returnvalue) 1e+02 _returnvalue_3))
          (for _array_element _outoverlappingactors
            (Class|NDamageGameplayAbility|CauseDamage _array_element))
          (Ability|EndAbility))))
    (:OnCancelled
      (Ability|EndAbility))))