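; GA_Heal is a gameplay ability that heals its owning character through an animated, stationary cast.
; On activation it commits the cost, saves and zeroes walk speed, and plays the heal montage supplied by the avatar.
; A Montage.Heal gameplay event applies GE_Heal to the owner.
; Montage completion, interruption or cancellation restores the saved speed, commits the cooldown and ends the ability.
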(event Ability|EventActivateAbility
  (Ability|CommitAbilityCost false)
  (bind _asncharacter_base (Utilities|Casting|CastToNCharacterBase (Ability|GetAvatarActorfromActorInfo)))
  (Variables|Default|SetDefaultWalkSpeed (Class|MovementComponent|GetMaxSpeed (Variables|/Script/Engine.Character|GetCharacterMovement _asncharacter_base)))
  (Variables|Default|SetCharacter%20Movement (Variables|/Script/Engine.Character|GetCharacterMovement _asncharacter_base))
  (Variables|/Script/Engine.CharacterMovementComponent|SetMaxWalkSpeed (Variables|/Script/Engine.Character|GetCharacterMovement _asncharacter_base) 0.0)
  (bind _returnvalue (Class|CombatInterface|GetHealMontage(Message) (Ability|GetAvatarActorfromActorInfo)))
  (|PlayMontageandWaitProxy "None" _returnvalue 1.0 "None" true 1.0 0.0 false
    (:then
      (Ability|Tasks|WaitGameplayEvent "(TagName=\"Montage.Heal\")" 0
        (:EventReceived
          (Ability|ApplyGameplayEffectToOwner "/Game/Blueprints/AbilitySystem/GameplayAbilities/Heal/GE_Heal.GE_Heal_C"))))
    (:OnCompleted
      (Variables|/Script/Engine.CharacterMovementComponent|SetMaxWalkSpeed (Variables|Default|GetCharacter%20Movement) (Variables|Default|GetDefaultWalkSpeed) :!label _label)
      (Ability|CommitAbilityCooldown false)
      (Ability|EndAbility))
    (:OnInterrupted
      (goto _label))
    (:OnCancelled
      (goto _label))))