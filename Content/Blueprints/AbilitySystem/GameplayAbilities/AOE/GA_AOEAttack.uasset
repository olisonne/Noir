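; Gameplay ability for an area-of-effect attack that damages actors around the avatar.
; On activation it commits, stops walking by zeroing max walk speed, and plays a montage supplied by the avatar through an interface message.
; A Montage.Attack.AOE gameplay event times the hit, which sphere-overlaps around the avatar, excluding itself, and calls CauseDamage on each result.
; Montage completion, interruption or cancellation restores the saved speed and ends the ability.
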(event Ability|EventActivateAbility
  (bind _returnvalue (Ability|GetAvatarActorfromActorInfo))
  (Ability|CommitAbility)
  (bind _asncharacter_base (Utilities|Casting|CastToNCharacterBase (Ability|GetAvatarActorfromActorInfo)))
  (Variables|Default|SetDefaultWalkSpeed (Class|MovementComponent|GetMaxSpeed (Variables|/Script/Engine.Character|GetCharacterMovement _asncharacter_base)))
  (Variables|Default|SetCharacter%20Movement (Variables|/Script/Engine.Character|GetCharacterMovement _asncharacter_base))
  (Variables|/Script/Engine.CharacterMovementComponent|SetMaxWalkSpeed (Variables|/Script/Engine.Character|GetCharacterMovement _asncharacter_base) 0.0)
  (bind _returnvalue_2 (Class|CombatInterface|GetAOEAttackMontage(Message) _returnvalue))
  (|PlayMontageandWaitProxy "None" _returnvalue_2 1.0 "None" true 1.0 0.0 false
    (:then
      (Ability|Tasks|WaitGameplayEvent "(TagName=\"Montage.Attack.AOE\")" 0
        (:EventReceived
          (bind _outactors (Collision|SphereOverlapActors (Transformation|GetActorLocation _returnvalue) 5e+02 (Variables|Default|GetObject%20Types) 0 (Utilities|Array|MakeArray (Ability|GetAvatarActorfromActorInfo))))
          (for _array_element _outactors
            (Class|NDamageGameplayAbility|CauseDamage _array_element)))))
    (:OnCompleted
      (Variables|/Script/Engine.CharacterMovementComponent|SetMaxWalkSpeed (Variables|Default|GetCharacter%20Movement) (Variables|Default|GetDefaultWalkSpeed) :!label _label)
      (Ability|EndAbility))
    (:OnInterrupted
      (goto _label))
    (:OnCancelled
      (goto _label))))

(event Ability|EventOnEndAbility
  (params (bWasCancelled :type Boolean)))