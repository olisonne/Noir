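; GA_Bullet is a gameplay ability that fires a projectile at the location of player pawn 0.
; On activation it commits, gets the avatar's attack montages through interface messages and plays a random tagged one.
; When a gameplay event matching the montage's tag arrives, it queries the combat socket location and calls SpawnProjectile with the player's XY and a fixed height.
; The socket result is not wired onward, and the graph never calls EndAbility.
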(event Ability|EventActivateAbility
  (bind _returnvalue (Game|Player|GetPlayerPawn 0))
  (bind _returnvalue_2 (Transformation|GetActorLocation _returnvalue))
  (bind (_x _y) (Math|Vector|BreakVector _returnvalue_2))
  (Ability|CommitAbility)
  (bind _returnvalue_3 (Class|CombatInterface|GetAttackMontages(Message) (Ability|GetAvatarActorfromActorInfo)))
  (bind _output_get (Variables|Default|SetMontageData (Class|NDamageGameplayAbility|GetRandomTaggedMontagefromArray _returnvalue_3)))
  (|PlayMontageandWaitProxy "None" (.Montage (Utilities|Struct|BreakTaggedMontage _output_get)) 1.0 "None" false 1.0 0.0 false
    (:then
      (Ability|Tasks|WaitGameplayEvent (.MontageTag (Utilities|Struct|BreakTaggedMontage _output_get)) 0
        (:EventReceived
          (Class|CombatInterface|GetCombatSocketLocation(Message) (Ability|GetAvatarActorfromActorInfo) (.MontageTag (Utilities|Struct|BreakTaggedMontage _output_get)))
          (Class|NProjectileSpell|SpawnProjectile (Math|Vector|MakeVector _x _y 1.2e+02)))))))