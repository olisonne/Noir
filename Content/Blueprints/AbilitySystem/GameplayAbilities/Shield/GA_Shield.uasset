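; Gameplay Ability that gives the avatar a temporary shield.
; On activation it commits the cost, spawns a BP_Shield owned by the avatar and snap-attaches it to the avatar with the "root" socket name.
; After a Duration delay it destroys the shield and ends the ability, committing the cooldown only afterward, so cooldown timing starts when the shield expires.
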(event Ability|EventActivateAbility
  (bind _returnvalue (Ability|GetAvatarActorfromActorInfo))
  (bind _returnvalue_2 (Transformation|GetActorLocation _returnvalue))
  (Ability|CommitAbilityCost false)
  (bind _returnvalue_3 (Game|SpawnActorfromClass "/Game/Blueprints/Actor/Shield/BP_Shield.BP_Shield_C" (Math|Transform|MakeTransform (Math|Vector|MakeVector (.x _returnvalue_2) (.y _returnvalue_2) (- (.z _returnvalue_2) 4e+01))) "AlwaysSpawn" "MultiplyWithRoot" (Ability|GetAvatarActorfromActorInfo) 0))
  (Variables|Default|SetShield _returnvalue_3)
  (Transformation|AttachActorToActor _returnvalue_3 (Ability|GetAvatarActorfromActorInfo) "root" "SnapToTarget" "SnapToTarget" "SnapToTarget" false)
  (Utilities|FlowControl|Delay (Variables|Default|GetDuration))
  (Actor|DestroyActor (Variables|Default|GetShield))
  (Ability|EndAbility)
  (Ability|CommitAbilityCooldown false))